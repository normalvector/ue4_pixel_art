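; Palette maker Blueprint that builds a one-pixel-high palette render target from a color array when constructed, using five hard-coded test colors.
; MakePalette sizes the width to the next power of two and clears it to black.
; It then draws one UV-bounded square per entry with a dynamic material, feeding the target back as source texture.
; Each square currently receives the same constant color instead of its array entry.
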(event EventBeginPlay)

(event Collision|EventActorBeginOverlap
  (params (OtherActor :type Actor%20Object%20Reference)))

(event EventTick
  (params (DeltaSeconds :type Float%20%28single-precision%29)))

(fn ConstructionScript
  (CallFunction|MakePalette (Utilities|Array|MakeArray (Utilities|Struct|MakeLinearColor 0.0 0.0 0.0 0.0) (Utilities|Struct|MakeLinearColor 1.0 1.0 1.0 0.0) (Utilities|Struct|MakeLinearColor 1.0 0.0 0.0 0.0) (Utilities|Struct|MakeLinearColor 0.0 1.0 0.0 0.0) (Utilities|Struct|MakeLinearColor 0.0 0.0 1.0 0.0))))

(fn NextPowerOfTwo
  (params (Value :type Integer))
  (LocalVariables|SetNextPower 0)
  (while (> Value (Math|Float|Truncate (Math|Float|Power 2.0 (Math|Conversions|ToFloat(Integer) (LocalVariables|GetNextPower)))))
    (Math|Integer|IncrementInt (LocalVariables|GetNextPower)))
  (return (Math|Float|Truncate (Math|Float|Power 2.0 (Math|Conversions|ToFloat(Integer) (LocalVariables|GetNextPower))))))

(fn MakePalette
  (params (Colors :type Array%20of%20Linear%20Color%20Structures))
  (bind _returnvalue (Utilities|Array|Length Colors))
  (bind _nextpoweroftwo (CallFunction|NextPowerOfTwo _returnvalue))
  (bind _returnvalue_2 (Math|Conversions|ToFloat(Integer) _nextpoweroftwo))
  (bind _returnvalue_3 (Rendering|CreateRenderTarget2D _nextpoweroftwo 1))
  (bind _output_get (Variables|Default|SetTextureRenderTarget _returnvalue_3))
  (Variables|/Script/Engine.Texture|SetCompressionNoAlpha _output_get true)
  (Variables|/Script/Engine.Texture|SetCompressionSettings _output_get "TC_EditorIcon")
  (Variables|/Script/Engine.Texture|SetLODGroup (Variables|Default|GetTextureRenderTarget) "TEXTUREGROUP_Pixels2D")
  (Rendering|DrawMaterialtoRenderTarget (Variables|Default|GetTextureRenderTarget) "/Game/render_pixel_art/palette_maker/fill_with_black_m.fill_with_black_m")
  (bind _returnvalue_4 (Rendering|Material|CreateDynamicMaterialInstance "/Game/render_pixel_art/palette_maker/square_renderer_m.square_renderer_m" :!class /Script/Engine.KismetMaterialLibrary))
  (Variables|Default|SetSquareRendererDMI _returnvalue_4)
  (for (_ _array_index) Colors
    (Rendering|Material|SetVectorParameterValue (Variables|Default|GetSquareRendererDMI) "Color" (Utilities|Struct|MakeLinearColor 0.5 1.0 0.0 0.0) :!class /Script/Engine.MaterialInstanceDynamic)
    (Rendering|Material|SetVectorParameterValue (Variables|Default|GetSquareRendererDMI) "MinUV" (Utilities|Struct|MakeLinearColor (|((1/size)*index) _returnvalue_2 (Math|Conversions|ToFloat(Integer) _array_index)) 0.0 0.0 0.0) :!class /Script/Engine.MaterialInstanceDynamic)
    (Rendering|Material|SetVectorParameterValue (Variables|Default|GetSquareRendererDMI) "MaxUV" (Utilities|Struct|MakeLinearColor (|((1/size)*(index*1)) _returnvalue_2 (Math|Conversions|ToFloat(Integer) _array_index)) 1.0 0.0 0.0) :!class /Script/Engine.MaterialInstanceDynamic)
    (Rendering|Material|SetTextureParameterValue (Variables|Default|GetSquareRendererDMI) "SrcTexture" (Variables|Default|GetTextureRenderTarget))
    (Rendering|DrawMaterialtoRenderTarget (Variables|Default|GetTextureRenderTarget) (Variables|Default|GetSquareRendererDMI)))
  (return (Variables|Default|GetTextureRenderTarget)))